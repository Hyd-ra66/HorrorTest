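; BP_SpeedMeter is a dial instrument that shows a normalized speed value by rotating its Arrow's yaw.
; On BeginPlay it registers itself with the BP_Harvester found in the level and zeroes the needle.
; SetValue maps the value to the needle angle, and ResetSpeedMeter uses a timeline to ease it back to zero.
; A self-calling, delayed Random event jitters the needle around the stored value over a narrower angular range while IsRandomActive is set.
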(event Custom|SetValue
  (params (Value :type Float%20%28double-precision%29))
  (Variables|Default|SetValue Value)
  (Transformation|SetRelativeRotation (Variables|Default|GetArrow) (Math|Rotator|MakeRotator 0.0 0.0 (Math|Float|MapRangeUnclamped Value 0.0 1.0 -75.0 75.0)) false false))

(event Custom|Random
  (if (Variables|Default|GetIsRandomActive)
    (Utilities|FlowControl|Delay (Math|Random|RandomFloatinRange 0.05 0.1))
    (bind _output_get (Variables|Default|SetTempValue (Math|Float|Clamp(Float) (+ (Variables|Default|GetValue) (Math|Random|RandomFloatinRange (* (Variables|Default|GetRandomRange) -1.0) (Variables|Default|GetRandomRange))) (- (Variables|Default|GetValue) (Variables|Default|GetRandomRange)) (+ (Variables|Default|GetValue) (Variables|Default|GetRandomRange)))))
    (Transformation|SetRelativeRotation (Variables|Default|GetArrow) (Math|Rotator|MakeRotator 0.0 0.0 (Math|Float|MapRangeUnclamped _output_get 0.0 1.0 -55.0 55.0)) false false)
    (CallFunction|Random)))

(event Custom|ResetSpeedMeter
  (bind _newtrack_0 (Timeline|ResetTimeline PlayFromStart)
    (:Update
      (CallFunction|SetValue (Math|Float|Lerp (Variables|Default|GetValue) 0.0 _newtrack_0)))))

(event EventBeginPlay
  (bind _returnvalue (Actor|GetActorOfClass "/Game/Blueprints/Harvester/BP_Harvester.BP_Harvester_C"))
  (Utilities|IsValid _returnvalue
    (:Is%20Valid
      (bind _output_get (Variables|Default|SetHarvesterRef _returnvalue))
      (Variables|/Game/Blueprints/Harvester/BP_Harvester.BP_Harvester_C|SetSpeedMeterRef _output_get self)
      (CallFunction|SetValue 0.0))))

(fn ConstructionScript)