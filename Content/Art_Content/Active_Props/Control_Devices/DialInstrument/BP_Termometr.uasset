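; BP_Termometr is a thermometer dial prop that shows a None, Low, Medium or High level by rotating its Arrow.
; On BeginPlay it finds BP_Harvester, registers itself as that actor's TermometrRef and, if found, starts at None.
; SetValueByType snaps the arrow's yaw to the matching preset, with None sharing Low's, and ResetIndicator returns to None.
; SetValue is an empty event, and the Set and Reset timeline animations are never run.
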(event Custom|SetValue
  (params (Value :type Float%20%28double-precision%29)))

(event Custom|ResetIndicator
  (CallFunction|SetValuebyType "NewEnumerator3"))

(event Custom|SetValueByType
  (params (ValueType :type E_ValueType%20Enum :default "NewEnumerator3"))
  (switch Utilities|FlowControl|Switch|SwitchonE_ValueType ValueType
    (:NewEnumerator3
      (Variables|Default|SetValueToSet (Variables|Default|GetLowValue) :!label _label))
    (:NewEnumerator0
      (goto _label))
    (:NewEnumerator1
      (Variables|Default|SetValueToSet (Variables|Default|GetMiddleValue)))
    (:NewEnumerator2
      (Variables|Default|SetValueToSet (Variables|Default|GetHighValue))))
  (CallFunction|SetValue (Variables|Default|GetValueToSet))
  (Transformation|SetRelativeRotation (Variables|Default|GetArrow) (Math|Rotator|MakeRotator 0.0 0.0 (Variables|Default|GetValueToSet)) false false))

(event EventBeginPlay
  (bind _returnvalue (Actor|GetActorOfClass "/Game/Blueprints/Harvester/BP_Harvester.BP_Harvester_C"))
  (Utilities|IsValid _returnvalue
    (:Is%20Valid
      (bind _output_get (Variables|Default|SetHarvesterRef _returnvalue))
      (Variables|/Game/Blueprints/Harvester/BP_Harvester.BP_Harvester_C|SetTermometrRef _output_get self)
      (CallFunction|SetValuebyType "NewEnumerator3"))))

(fn ConstructionScript)