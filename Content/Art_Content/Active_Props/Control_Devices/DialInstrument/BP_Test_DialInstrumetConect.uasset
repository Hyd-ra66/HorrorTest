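; Test dial instrument prop that turns its arrow mesh to show a value and makes the needle jitter continuously.
; SetValue stores the value and linearly maps a 0–1 input to the arrow's relative yaw across a symmetric arc.
; From BeginPlay, which sets full scale, the Random event re-triggers itself after short random delays, offsetting the needle within RandomRange of the stored value without changing it.
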(event Custom|SetValue
  (params (Value :type Float%20%28double-precision%29))
  (Variables|Default|SetValue Value)
  (Transformation|SetRelativeRotation (Variables|Default|GetSM_DialInstrument_SM_DialInstrument_Arrow) (Math|Rotator|MakeRotator 0.0 0.0 (Math|Float|MapRangeUnclamped Value 0.0 1.0 -55.0 55.0)) false false))

(event Custom|Random
  (Utilities|FlowControl|Delay (Math|Random|RandomFloatinRange 0.01 0.1))
  (bind _output_get (Variables|Default|SetTempValue (Math|Float|Clamp(Float) (+ (Variables|Default|GetValue) (Math|Random|RandomFloatinRange (* (Variables|Default|GetRandomRange) -1.0) (Variables|Default|GetRandomRange))) (- (Variables|Default|GetValue) (Variables|Default|GetRandomRange)) (+ (Variables|Default|GetValue) (Variables|Default|GetRandomRange)))))
  (Transformation|SetRelativeRotation (Variables|Default|GetSM_DialInstrument_SM_DialInstrument_Arrow) (Math|Rotator|MakeRotator 0.0 0.0 (Math|Float|MapRangeUnclamped _output_get 0.0 1.0 -55.0 55.0)) false false)
  (CallFunction|Random))

(event EventBeginPlay
  (CallFunction|SetValue 1.0)
  (CallFunction|Random))

(fn ConstructionScript)