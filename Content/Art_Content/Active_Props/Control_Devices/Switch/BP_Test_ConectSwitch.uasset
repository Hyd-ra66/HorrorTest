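; Interactable switch prop that toggles between Engine and Probe modes, each gated by an enabled flag.
; On BeginPlay it registers itself with BP_Harvester and creates dynamic materials for both decals.
; Interacting rotates the lever and plays a sound.
; Switching to Probe also runs a timed "Zond" analysis with W_ZondText status messages and notifies the Harvester when analysis completes.
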(event Custom|SwitchToProbe
  (if (Variables|Default|GetProbeEnabled)
    (Transformation|SetRelativeRotation (Variables|Default|GetSwitch_Switch) "0.000000,30.000000,0.000000" false false)
    (Audio|PlaySound2D (Variables|Default|GetSound) 1.0 1.0 0.0 0 0)
    (Variables|Default|SetEngineOn false)
    (CallFunction|StartProbe)))

(event Custom|SwitchToEngine
  (if (Variables|Default|GetEngineEnabled)
    (Transformation|SetRelativeRotation (Variables|Default|GetSwitch_Switch) "0.000000,-30.000000,0.000000" false false)
    (Audio|PlaySound2D (Variables|Default|GetSound) 1.0 1.0 0.0 0 0)
    (Variables|Default|SetEngineOn true)))

(event Custom|OnInteract
  (if (Variables|Default|GetEngineOn)
    (CallFunction|SwitchtoProbe)
    (else
      (CallFunction|SwitchtoEngine))))

(event Custom|StartProbe
  (bind _zondwidget (Variables|Default|GetZondWidget))
  (CallFunction|CreateWidget)
  (Default|SetText (Variables|Default|GetZondWidget) "Zond is running...")
  (Utilities|FlowControl|Delay (Math|Random|RandomFloatinRange 5.0 7.0))
  (Default|SetText (Variables|Default|GetZondWidget) "Analizing")
  (Utilities|FlowControl|Delay 5.0)
  (Default|SetText (Variables|Default|GetZondWidget) "Analize complete!")
  (Default|AnalizeComplete (Variables|Default|GetHarvesterRef))
  (Utilities|FlowControl|Delay 2.0)
  (Utilities|IsValid _zondwidget
    (:Is%20Valid
      (Widget|RemovefromParent _zondwidget))))

(event EventBeginPlay
  (bind _returnvalue (Actor|GetActorOfClass "/Game/Blueprints/Harvester/BP_Harvester.BP_Harvester_C"))
  (bind _output_get (Variables|Default|SetHarvesterRef _returnvalue))
  (Variables|/Game/Blueprints/Harvester/BP_Harvester.BP_Harvester_C|SetSwitchRef _output_get self)
  (Utilities|FlowControl|Sequence
    (:then_0
      (bind _returnvalue_2 (Rendering|Material|CreateDynamicMaterialInstance (Variables|Default|GetEngineDecal) :!class /Script/Engine.DecalComponent))
      (Variables|Default|SetEngineDecalMID _returnvalue_2))
    (:then_1
      (bind _returnvalue_3 (Rendering|Material|CreateDynamicMaterialInstance (Variables|Default|GetProbeDecal) :!class /Script/Engine.DecalComponent))
      (Variables|Default|SetProbeDecalMID _returnvalue_3))))

(fn ConstructionScript)

(fn CreateWidget
  (bind _returnvalue (UserInterface|CreateWidget "/Game/Widgets/W_ZondText.W_ZondText_C" (Game|GetPlayerController 0)))
  (bind _output_get (Variables|Default|SetZondWidget _returnvalue))
  (UserInterface|Viewport|AddtoViewport _output_get 0))