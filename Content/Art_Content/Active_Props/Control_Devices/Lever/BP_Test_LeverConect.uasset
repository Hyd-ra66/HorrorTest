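; Interactable three-position lever that sets the Harvester's LeverValue during travel.
; On BeginPlay it finds BP_Harvester and registers itself as TravelLeverRef.
; Interaction, allowed only while traveling with acceleration finished, steps through Medium, alternating between Low and High on each move away from center.
; SetState rotates the mesh, writes a negative, zero or positive value to the Harvester and plays a sound; ResetLever recenters it.
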(event Custom|ChangeState
  (switch Utilities|FlowControl|Switch|SwitchonE_EngineState (Variables|Default|GetCurrentState)
    (:NewEnumerator0
      (switch Utilities|FlowControl|Switch|SwitchonE_EngineState (Variables|Default|GetPreviousSide)
        (:NewEnumerator1
          (Variables|Default|SetPreviousSide "NewEnumerator2")
          (CallFunction|SetState "NewEnumerator2"))
        (:NewEnumerator2
          (Variables|Default|SetPreviousSide "NewEnumerator1")
          (CallFunction|SetState "NewEnumerator1"))))
    (:NewEnumerator1
      (CallFunction|SetState "NewEnumerator0" :!label _label))
    (:NewEnumerator2
      (goto _label))))

(event Custom|SetState
  (params (NewParam :type E_EngineState%20Enum :default "NewEnumerator0"))
  (bind _output_get (Variables|Default|SetCurrentState NewParam))
  (switch Utilities|FlowControl|Switch|SwitchonE_EngineState _output_get
    (:NewEnumerator0
      (Transformation|SetRelativeRotation (Variables|Default|GetSM_Lever) "0, 0, 0" false false)
      (Variables|/Game/Blueprints/Harvester/BP_Harvester.BP_Harvester_C|SetLeverValue (Variables|Default|GetHarvesterRef) 0.0))
    (:NewEnumerator1
      (Transformation|SetRelativeRotation (Variables|Default|GetSM_Lever) "-40.000000,0.000000,0.000000" false false)
      (Variables|/Game/Blueprints/Harvester/BP_Harvester.BP_Harvester_C|SetLeverValue (Variables|Default|GetHarvesterRef) -5.0))
    (:NewEnumerator2
      (Transformation|SetRelativeRotation (Variables|Default|GetSM_Lever) "40.000000,0.000000,0.000000" false false)
      (Variables|/Game/Blueprints/Harvester/BP_Harvester.BP_Harvester_C|SetLeverValue (Variables|Default|GetHarvesterRef) 5.0)))
  (Audio|PlaySound2D (Variables|Default|GetSound) 1.0 1.0 0.0 0 0))

(event Custom|OnInteract
  (if (and (Variables|/Game/Blueprints/Harvester/BP_Harvester.BP_Harvester_C|GetIsTraveling (Variables|Default|GetHarvesterRef)) (Variables|/Game/Blueprints/Harvester/BP_Harvester.BP_Harvester_C|GetAccelerationFinished (Variables|Default|GetHarvesterRef)))
    (CallFunction|ChangeState)))

(event Custom|ResetLever
  (CallFunction|SetState "NewEnumerator0"))

(event EventBeginPlay
  (bind _returnvalue (Actor|GetActorOfClass "/Game/Blueprints/Harvester/BP_Harvester.BP_Harvester_C"))
  (bind _output_get (Variables|Default|SetHarvesterRef _returnvalue))
  (Variables|/Game/Blueprints/Harvester/BP_Harvester.BP_Harvester_C|SetTravelLeverRef _output_get self)
  (Variables|Default|SetPreviousSide "NewEnumerator2")
  (Variables|Default|SetCurrentState "NewEnumerator0"))

(fn ConstructionScript)