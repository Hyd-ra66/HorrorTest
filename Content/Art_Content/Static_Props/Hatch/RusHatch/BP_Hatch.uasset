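; BP_Hatch is a Russian-style hatch prop that bursts open when its EndGame event fires.
; EndGame enables physics and gravity on the two cylinder pieces and the door, then launches them with impulses.
; After a brief delay it assigns a smoke particle effect and moves it along a spline via a timeline.
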(event Custom|EndGame
  (bind _sm_hatch_body_sm_hatch_cyl1 (Variables|Default|GetSM_Hatch_Body_SM_Hatch_Cyl1))
  (bind _sm_hatch_door (Variables|Default|GetSM_Hatch_Door))
  (Physics|SetSimulatePhysics _sm_hatch_body_sm_hatch_cyl1 true)
  (Physics|SetEnableGravity _sm_hatch_body_sm_hatch_cyl1 true)
  (Physics|AddImpulse _sm_hatch_body_sm_hatch_cyl1 "0.000000,200.000000,0.000000" "None" true)
  (Physics|AddImpulseatLocation _sm_hatch_door "0.000000,40000.000000,0.000000" (Transformation|GetWorldLocation _sm_hatch_door) "None")
  (Utilities|FlowControl|Delay 0.12)
  (Class|NiagaraComponent|SetAsset (Variables|Default|GetP_Smoke_07) "/Game/HarvesterHorror/Fx/Niagara/Smoke/P_Smoke_07.P_Smoke_07" true)
  (bind _newtrack_0 (Timeline|Timeline PlayFromStart)
    (:Update
      (Transformation|SetRelativeLocation (Variables|Default|GetP_Smoke_07) (Spline|GetLocationatTime (Variables|Default|GetSpline) _newtrack_0 "Local" false) false false))))

(event EventBeginPlay)

(event Collision|EventActorBeginOverlap
  (params (OtherActor :type Actor%20Object%20Reference)))

(event EventTick
  (params (DeltaSeconds :type Float%20%28single-precision%29)))

(fn ConstructionScript)