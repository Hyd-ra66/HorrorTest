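; Interactable radio prop that switches between two sounds with a silent middle position, sliding its frequency knob to match.
; BeginPlay starts the first sound at the top knob position.
; Each OnInteract advances a Low/Medium/High state machine, using PreviousState to alternate which sound follows the silent step.
; SpawnSound plays audio at the actor with radio attenuation and keeps the component reference so it can be deactivated.
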(event Custom|OnInteract
  (bind _soundref (Variables|Default|GetSoundRef))
  (bind _soundref_2 (Variables|Default|GetSoundRef))
  (switch Utilities|FlowControl|Switch|SwitchonE_EngineState (Variables|Default|GetState)
    (:NewEnumerator0
      (switch Utilities|FlowControl|Switch|SwitchonE_EngineState (Variables|Default|GetPreviousState)
        (:NewEnumerator1
          (Utilities|IsValid _soundref
            (:Is%20Valid
              (Components|Activation|Deactivate _soundref))
            (:Is%20Not%20Valid
              _))
          (CallFunction|SpawnSound (Variables|Default|GetSound1))
          (Transformation|SetRelativeLocation (Variables|Default|GetSM_Radio_FrequencyKnob) "0.000000,20.000000,29.000000" false false)
          (Variables|Default|SetPreviousState "NewEnumerator2")
          (Variables|Default|SetState "NewEnumerator1"))
        (:NewEnumerator2
          (Utilities|IsValid _soundref_2
            (:Is%20Valid
              (Components|Activation|Deactivate _soundref_2))
            (:Is%20Not%20Valid
              _))
          (CallFunction|SpawnSound (Variables|Default|GetSound2))
          (Transformation|SetRelativeLocation (Variables|Default|GetSM_Radio_FrequencyKnob) "0.000000,20.000000,21.000000" false false)
          (Variables|Default|SetPreviousState "NewEnumerator1")
          (Variables|Default|SetState "NewEnumerator2"))))
    (:NewEnumerator1
      (Variables|Default|SetState "NewEnumerator0" :!label _label)
      (Components|Activation|Deactivate (Variables|Default|GetSoundRef))
      (Transformation|SetRelativeLocation (Variables|Default|GetSM_Radio_FrequencyKnob) "0.000000,20.000000,25.000000" false false))
    (:NewEnumerator2
      (goto _label))))

(event EventBeginPlay
  (Variables|Default|SetState "NewEnumerator2")
  (CallFunction|SpawnSound (Variables|Default|GetSound1))
  (Transformation|SetRelativeLocation (Variables|Default|GetSM_Radio_FrequencyKnob) "0.000000,20.000000,29.000000" false false)
  (Variables|Default|SetPreviousState "NewEnumerator2"))

(fn ConstructionScript)

(fn SpawnSound
  (params (Sound :type Sound%20Base%20Object%20Reference))
  (bind _returnvalue (Audio|SpawnSoundatLocation Sound (Transformation|GetActorLocation) "0, 0, 0" 1.0 1.0 0.0 "/Game/Audio/SA_Radio.SA_Radio" 0))
  (Variables|Default|SetSoundRef _returnvalue))