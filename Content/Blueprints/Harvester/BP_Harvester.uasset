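; Harvester controller that drives timed trips to well points and reveals the item found at each.
; A data table defines each path's surface segments and item; Tick counts down distance, with surface and lever setting speed.
; Recursive delay timers update progress and drain fuel, feeding screen widgets and in-world gauges.
; Arrival resets controls and enables the probe; completed analysis shows temperature, density and activity, then spawns the item.
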(event Custom|StartTravel
  ;[0.04501 0.3754 1] Start travel event
  (if (and (Variables|Default|GetUtilizationDone) (not (Variables|/Game/Blueprints/Harvester/BP_Door.BP_Door_C|GetIsOpen (Variables|/Game/Blueprints/Controls/BP_DoorControl.BP_DoorControl_C|GetDoorRef (Variables|Default|GetDoorControlRef)))))
    (Variables|Default|SetUtilizationDone false)
    (CallFunction|Acceleration)
    (Variables|Default|SetIsTraveling true)
    (CallFunction|ProgressTimer)
    (CallFunction|FueelTimer)
    (bind _returnvalue (Audio|SpawnSound2D (Variables|Default|GetEngineSound) 1.0 1.0 0.0 0))
    (Variables|Default|SetEngineSoundObject _returnvalue)
    (CallFunction|PlayCameraShake)
    (Variables|/Game/Blueprints/Controls/BP_DoorControl.BP_DoorControl_C|SetIsControlEnabled (Variables|Default|GetDoorControlRef) false)
    (Default|SetDistance (Variables|Default|GetDistanceWidget) (Utilities|Text|ToText(Float) (Variables|Default|GetCurrentDistanceToPoint) "HalfToEven"))))

(event Custom|Acceleration
  (bind _speedmeterref (Variables|Default|GetSpeedMeterRef))
  ;[0.4146 0.4121 1] Acceleration
  (Variables|Default|SetAccelerationFinished false)
  (CallFunction|SetSpeedbySurface)
  (bind _newtrack_0 (Timeline|AccelerationTimeline PlayFromStart)
    (:Update
      (bind _output_get (Variables|Default|SetCurrentSpeed (Math|Float|Lerp 0.0 (Variables|Default|GetMaxSpeed) _newtrack_0)))
      (Default|SetValue (Variables|Default|GetSpeedMeterRef) (Math|Float|MapRangeClamped _output_get 0.0 35.0 0.0 1.0)))
    (:Finished
      (Variables|Default|SetAccelerationFinished true)
      (Variables|/Game/Art_Content/Active_Props/Control_Devices/DialInstrument/BP_SpeedMeter.BP_SpeedMeter_C|SetIsRandomActive _speedmeterref true)
      (Default|Random _speedmeterref))))

(event Custom|PointReached
  ;[0.4509 1 0.394] Point reached event
  (Variables|Default|SetIsTraveling false)
  (Math|Integer|IncrementInt (Variables|Default|GetCurrentPathIndex)
    (:%20%20
      (Default|RevertControl (Variables|Default|GetTravelControlRef))
      (Default|SetProbeActive (Variables|Default|GetSwitchRef) true)
      (Default|ResetSpeedMeter (Variables|Default|GetSpeedMeterRef))
      (Audio|PlaySound2D (Variables|Horror|GetReachPointSound) 1.0 1.0 0.0 0 0)
      (Components|Activation|Deactivate (Variables|Default|GetEngineSoundObject))
      (Variables|/Game/Art_Content/Active_Props/Control_Devices/DialInstrument/BP_SpeedMeter.BP_SpeedMeter_C|SetIsRandomActive (Variables|Default|GetSpeedMeterRef) false)
      (Default|ResetLever (Variables|Default|GetTravelLeverRef))
      (CallFunction|PlayCameraShake)
      (bind _result (Math|Integer|DecrementInt (Variables|Default|GetWellRemainCount))
        (:%20%20
          (Default|SetCount (Variables|Default|GetWellRemainWidget) (Utilities|Text|ToText(Integer) _result)))))))

(event Custom|ProgressTimer
  ;[0.9662 1 0.02144] Progress timer
  (Utilities|FlowControl|Delay 1.0)
  (bind _result (Math|Integer|IncrementInt (Variables|Default|GetProgressValue))
    (:%20%20
      (Default|SetProgress (Variables|Default|GetProgressWidget) (Utilities|Text|ToText(Integer) _result))
      (if (Variables|Default|GetIsTraveling)
        (CallFunction|ProgressTimer)))))

(event Custom|FueelTimer
  ;[1 0.9545 0.08121] Fuel timer
  (Utilities|FlowControl|Delay 1.0)
  (if (== (Variables|Default|GetCurrentSpeed) 2e+01)
    (Math|Integer|DecrementInt (Variables|Fuel|GetFuelValue)
      (:%20%20
        _))
    (else
      (Variables|Fuel|SetFuelValue (- (Variables|Fuel|GetFuelValue) 2))))
  (Utilities|FlowControl|Sequence
    (:then_0
      (for _array_element (Variables|Default|GetFuelIndicators)
        (Default|SetFuel _array_element (/ (Math|Conversions|ToFloat(Integer) (Variables|Fuel|GetFuelValue)) (Math|Conversions|ToFloat(Integer) (Variables|Fuel|GetMaxFuelValue))))
        (if (Variables|Default|GetIsTraveling)
          (CallFunction|FueelTimer))))
    (:then_1
      (Default|SetFuel (Variables|Default|GetSpeedWidget) (Utilities|Text|ToText(Integer) (Variables|Fuel|GetFuelValue))))))

(event Custom|AnalizeComplete
  ;[0.04144 1 0.2389] Analize complete event
  (Utilities|FlowControl|Sequence
    (:then_0
      ;;[1 1 1] Debug
      (Default|SetName (Variables|Default|GetItemValuesWidget) (Utilities|Text|ToText(String) (Utilities|String|EnumtoString (Variables|Default|GetItem)))))
    (:then_1
      (Default|SetValuebyType (Variables|Default|GetTermometrRef) (Variables|Default|GetTemperature))
      (Default|SetTemperature (Variables|Default|GetItemValuesWidget) (Utilities|Text|ToText(String) (Utilities|String|EnumtoString (Variables|Default|GetTemperature)))))
    (:then_2
      (Default|SetValuebyType (Variables|Default|GetDensityMeterRef) (Variables|Default|GetDensity))
      (Default|SetDensity (Variables|Default|GetItemValuesWidget) (Utilities|Text|ToText(String) (Utilities|String|EnumtoString (Variables|Default|GetDensity)))))
    (:then_3
      (Default|SetValuebyType (Variables|Default|GetActivityMeterRef) (Variables|Default|GetActivity))
      (Default|SetActivity (Variables|Default|GetItemValuesWidget) (Utilities|Text|ToText(String) (Utilities|String|EnumtoString (Variables|Default|GetActivity)))))
    (:then_4
      (bind _returnvalue (Game|SpawnActorfromClass "/Game/Blueprints/BP_Item.BP_Item_C" (Math|Transform|MakeTransform (Variables|Default|GetItemSpawnLocation)) "Undefined" "MultiplyWithRoot" 0 (Variables|Default|GetItemStatic%20Mesh) (Variables|Default|GetItemSkeletal%20Mesh) (Variables|Default|GetItemAnimation) 0))
      (Default|Init _returnvalue))))

(event Custom|Desinfection
  ;[1 0.2276 0.3576] Desinfection
  (bind _result (Math|Integer|DecrementInt (Variables|Default|GetDesinfectionPoints))
    (:%20%20
      (Development|PrintString (Utilities|String|Append (Utilities|String|ToString(Integer) _result) " Desinfection points"))
      (if (<= _result 0)
        (Variables|Default|SetDesinfectionPoints 0)
        (Variables|/Game/Blueprints/Controls/BP_Desinfection.BP_Desinfection_C|SetIsControlEnabled (Variables|Default|GetDesinfectionRef) false)))))

(event EventBeginPlay
  ;[0.1816 1 0.1744] Begin play
  (CallFunction|InitDT)
  (CallFunction|CreateWidgets)
  (CallFunction|InitPathData)
  (Utilities|FlowControl|DelayUntilNextTick)
  (bind _returnvalue (Actor|GetActorOfClass "/Game/Blueprints/Harvester/BP_ItemSpawnPoint.BP_ItemSpawnPoint_C"))
  (Variables|Default|SetItemSpawnLocation (Transformation|GetActorLocation _returnvalue))
  (bind _returnvalue_2 (Actor|GetActorOfClass "/Game/Blueprints/BP_FirstPersonCharacter.BP_FirstPersonCharacter_C"))
  (Variables|Default|SetPlayerRef _returnvalue_2)
  (Utilities|FlowControl|Sequence
    (:then_0
      (bind _outactors (Actor|GetAllActorsOfClass "/Game/Blueprints/Controls/BP_Utilization.BP_Utilization_C"))
      (Variables|Default|SetOut%20Actors _outactors))
    (:then_1
      (bind _outactors_2 (Actor|GetAllActorsOfClass "/Game/Art_Content/Active_Props/Control_Devices/Fuel_Indicator/BP_Test_FuelIndicatorConect.BP_Test_FuelIndicatorConect_C"))
      (bind _output_get (Variables|Default|SetFuelIndicators _outactors_2))
      (for _array_element _output_get
        (Default|SetFuel _array_element 1.0)))
    (:then_2
      (Variables|Default|SetUtilizationDone true))))

(event EventTick
  (params (DeltaSeconds :type Float%20%28single-precision%29))
  ;[1 0.4996 0.5195] Event tick
  (if (Variables|Default|GetIsTraveling)
    (CallFunction|CheckSurface)
    (if (Variables|Default|GetAccelerationFinished)
      (Variables|Default|SetCurrentSpeed (+ (Variables|Default|GetMaxSpeed) (Variables|Default|GetLeverValue)))
      (bind _output_get (Variables|Default|SetTraveledDistance (+ (* DeltaSeconds (/ (* (Variables|Default|GetCurrentSpeed) 1e+01) 3.6e+03)) (Variables|Default|GetTraveledDistance))))
      (bind _output_get_2 (Variables|Default|SetCurrentDistanceToPoint (- (Variables|Default|GetCurrentDistanceToPoint) _output_get)))
      (if (<= _output_get_2 0.0)
        (Default|SetDistance (Variables|Default|GetDistanceWidget) (Utilities|Text|ToText(Integer) (Math|Float|Round (Variables|Default|GetZeroFloat))))
        (CallFunction|PointReached)
        (else
          (Default|SetValue (Variables|Default|GetSpeedMeterRef) (Math|Float|MapRangeClamped (Variables|Default|GetCurrentSpeed) 0.0 35.0 0.0 1.0))
          ;[1 1 1] Comment
          (CallFunction|PrintDistanceandSpeed)))
      (else
        ;;[1 1 1] Comment
        (CallFunction|PrintDistanceandSpeed)))))

(fn ConstructionScript)

(fn InitDT
  (bind _outrownames (DataTable|GetDataTableRowNames (Variables|Default|GetPathsDataTable)))
  (bind _output_get (Variables|Default|SetPathNamesArray _outrownames))
  (Variables|Default|SetWellRemainCount (Utilities|Array|Length _output_get)))

(fn CreateWidgets
  (Utilities|FlowControl|Sequence
    (:then_0
      (bind _returnvalue (UserInterface|CreateWidget "/Game/Widgets/W_DistanceIndicator.W_DistanceIndicator_C" (Game|GetPlayerController 0)))
      (bind _output_get (Variables|Default|SetDistanceWidget _returnvalue))
      (UserInterface|Viewport|AddtoViewport _output_get 0))
    (:then_1
      (bind _returnvalue_2 (UserInterface|CreateWidget "/Game/Widgets/W_SpeedIndicator.W_SpeedIndicator_C" (Game|GetPlayerController 0)))
      (bind _output_get_2 (Variables|Default|SetSpeedWidget _returnvalue_2))
      (UserInterface|Viewport|AddtoViewport _output_get_2 0))
    (:then_2
      (bind _returnvalue_3 (UserInterface|CreateWidget "/Game/Widgets/W_ItemValues.W_ItemValues_C" (Game|GetPlayerController 0)))
      (bind _output_get_3 (Variables|Default|SetItemValuesWidget _returnvalue_3))
      (UserInterface|Viewport|AddtoViewport _output_get_3 0))
    (:then_3
      (bind _returnvalue_4 (UserInterface|CreateWidget "/Game/Widgets/W_Progress.W_Progress_C" (Game|GetPlayerController 0)))
      (bind _output_get_4 (Variables|Default|SetProgressWidget _returnvalue_4))
      (UserInterface|Viewport|AddtoViewport _output_get_4 0))
    (:then_4
      (bind _returnvalue_5 (UserInterface|CreateWidget "/Game/Widgets/W_WellRemainCount.W_WellRemainCount_C" (Game|GetPlayerController 0)))
      (bind _output_get_5 (Variables|Default|SetWellRemainWidget _returnvalue_5))
      (UserInterface|Viewport|AddtoViewport _output_get_5 0)
      (Default|SetCount (Variables|Default|GetWellRemainWidget) (Utilities|Text|ToText(Integer) (Variables|Default|GetWellRemainCount))))
    (:then_5
      (bind _returnvalue_6 (UserInterface|CreateWidget "/Game/Widgets/W_SurfaceType.W_SurfaceType_C" (Game|GetPlayerController 0)))
      (bind _output_get_6 (Variables|Default|SetSurfaceTypeWidget _returnvalue_6))
      (UserInterface|Viewport|AddtoViewport _output_get_6 0))))

(fn SetDecimalCount
  (params (A :type Float%20%28double-precision%29))
  (return (/ (Math|Conversions|ToFloat(Integer) (Math|Float|Truncate (* A 1e+01))) 1e+01)))

(fn CheckSurface
  (bind _surface_type (Variables|Surface|GetSurface%20Type))
  (bind _currentsurfaceindex (Variables|Default|GetCurrentSurfaceIndex))
  (bind _output (Utilities|Array|Get(acopy) _surface_type _currentsurfaceindex))
  (LocalVariables|SetLocal_TraveledDistance (- (Variables|Default|GetInitDistanceToPoint) (Variables|Default|GetCurrentDistanceToPoint)))
  (switch Utilities|FlowControl|Switch|SwitchonE_SurfaceType _output
    (:NewEnumerator0
      (Variables|Default|SetMaxSpeed 15.0))
    (:NewEnumerator1
      (Variables|Default|SetMaxSpeed 2e+01))
    (:NewEnumerator2
      (Variables|Default|SetMaxSpeed 25.0)))
  (if (>= (LocalVariables|GetLocal_TraveledDistance) (Utilities|Array|Get(acopy) (Variables|Surface|GetDistanceArray) (Variables|Default|GetCurrentSurfaceIndex)))
    (Math|Integer|IncrementInt (Variables|Default|GetCurrentSurfaceIndex)
      (:%20%20
        (CallFunction|PlayCameraShake)
        ;[1 1 1] Debug
        (Default|SetType (Variables|Default|GetSurfaceTypeWidget) (Utilities|Text|ToText(String) (Utilities|String|EnumtoString _output)))))))

(fn InitPathData
  (bind _surface_type (Variables|Surface|GetSurface%20Type))
  (bind _output (Utilities|Array|Get(acopy) _surface_type))
  (Utilities|Array|Clear (Variables|Surface|GetSurface%20Type))
  (Utilities|Array|Clear (Variables|Surface|GetDistanceArray))
  (bind _returnvalue (Utilities|GetDataTableRow (Variables|Default|GetPathsDataTable) (Utilities|Array|Get(acopy) (Variables|Default|GetPathNamesArray) (Variables|Default|GetCurrentPathIndex)))
    (:then
      (Variables|Default|SetItem (.PointItem (Utilities|Struct|BreakF_PathToPoint _returnvalue)))
      (Variables|Default|SetTemperature (.Temperature (Utilities|Struct|BreakF_PathToPoint _returnvalue)))
      (Variables|Default|SetDensity (.Density (Utilities|Struct|BreakF_PathToPoint _returnvalue)))
      (Variables|Default|SetActivity (.Activity (Utilities|Struct|BreakF_PathToPoint _returnvalue)))
      (Variables|Default|SetItemStatic%20Mesh (.StaticMesh (Utilities|Struct|BreakF_PathToPoint _returnvalue)))
      (Variables|Default|SetItemSkeletal%20Mesh (.SkeletalMesh (Utilities|Struct|BreakF_PathToPoint _returnvalue)))
      (Variables|Default|SetItemAnimation (.Animation (Utilities|Struct|BreakF_PathToPoint _returnvalue)))
      (for _array_element (.PathsArray (Utilities|Struct|BreakF_PathToPoint _returnvalue))
        (bind _output_get (Variables|Default|SetCurrentDistanceToPoint (+ (Variables|Default|GetCurrentDistanceToPoint) (.Length (Utilities|Struct|BreakF_GroundSurface _array_element)))))
        (Utilities|Array|Add (Variables|Surface|GetDistanceArray) _output_get)
        (Utilities|Array|Add (Variables|Surface|GetSurface%20Type) (.SurfaceType (Utilities|Struct|BreakF_GroundSurface _array_element)))
        (Variables|Default|SetCurrentSurfaceType _output)
        (Default|SetType (Variables|Default|GetSurfaceTypeWidget) (Utilities|Text|ToText(String) (Utilities|String|EnumtoString _output))))
      (Variables|Default|SetInitDistanceToPoint (Variables|Default|GetCurrentDistanceToPoint))
      (Variables|Default|SetCurrentSurfaceIndex 0))))

(fn SetSpeedbySurface
  (switch Utilities|FlowControl|Switch|SwitchonE_SurfaceType (Variables|Default|GetCurrentSurfaceType)
    (:NewEnumerator0
      (Variables|Default|SetMaxSpeed (- (Variables|Default|GetMaxSpeed) 5.0)))
    (:NewEnumerator2
      (Variables|Default|SetMaxSpeed (+ (Variables|Default|GetMaxSpeed) 5.0)))))

(fn PrintDistanceandSpeed
  (Default|SetDistance (Variables|Default|GetDistanceWidget) (Utilities|Text|ToText(Integer) (Math|Float|Round (Variables|Default|GetCurrentDistanceToPoint))))
  (Default|SetSpeed (Variables|Default|GetSpeedWidget) (Utilities|Text|ToText(Float) (CallFunction|SetDecimalCount (Variables|Default|GetCurrentSpeed)) "HalfToEven")))

(fn PlayCameraShake
  (Camera|PlayWorldCameraShake "/Game/Blueprints/BP_CameraShake.BP_CameraShake_C" (Transformation|GetActorLocation (Variables|Default|GetPlayerRef)) 0.0 5e+02))