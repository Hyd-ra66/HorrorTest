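; BP_Item is an item that attaches to a character's DropPoint when interacted with.
; Init applies whichever static mesh, skeletal mesh and animation assets are valid, playing the animation on a loop.
; OnInteract performs the attachment, snapping location and rotation to the DropPoint while keeping relative scale.
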(event Custom|Init
  (Utilities|FlowControl|Sequence
    (:then_0
      (Utilities|IsValid (Variables|Mesh|GetStaticMeshAsset)
        (:Is%20Valid
          (Components|StaticMesh|SetStaticMesh (Variables|Default|GetStaticMesh) (Variables|Mesh|GetStaticMeshAsset)))))
    (:then_1
      (Utilities|IsValid (Variables|Mesh|GetSkeletalMeshAsset)
        (:Is%20Valid
          (Components|SkeletalMesh|SetSkeletalMeshAsset (Variables|Default|GetSkeletalMesh) (Variables|Mesh|GetSkeletalMeshAsset)))))
    (:then_2
      (Utilities|IsValid (Variables|Mesh|GetAnimation)
        (:Is%20Valid
          (Components|Animation|PlayAnimation (Variables|Default|GetSkeletalMesh) (Variables|Mesh|GetAnimation) true))))))

(event Custom|OnInteract
  (params (CharacterRef :type BP%20First%20Person%20Character%20Object%20Reference))
  (Transformation|AttachComponentToComponent (Variables|/Game/Blueprints/BP_FirstPersonCharacter.BP_FirstPersonCharacter_C|GetDropPoint CharacterRef) "None" "SnapToTarget" "SnapToTarget" "KeepRelative" true))

(fn ConstructionScript)