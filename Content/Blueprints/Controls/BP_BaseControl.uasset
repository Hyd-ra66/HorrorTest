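; Base Blueprint for interactable controls tied to the harvester, providing shared setup, press feedback and animation hooks.
; On BeginPlay it finds the BP_Harvester and, if valid, caches it, its own starting location and every placed indicator matching the classes in IndicatorsToActivate.
; Interacting plays a 2D press sound.
; PlayAnimation forwards to an empty event, which, like the empty reversed-animation event, leaves the motion to child Blueprints.
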(event Custom|PlayAnimationEvent)

(event Custom|PlayReversedAnimation)

(event EventBeginPlay
  (bind _returnvalue (Actor|GetActorOfClass "/Game/Blueprints/Driving/BP_Harvester.BP_Harvester_C"))
  (Utilities|IsValid _returnvalue
    (:Is%20Valid
      (Variables|Default|SetHarvesterRef _returnvalue)
      (Variables|Horror|SetInitialLocation (Transformation|GetActorLocation))
      (for _array_element (Variables|Horror|GetIndicatorsToActivate)
        (bind _outactors (Actor|GetAllActorsOfClass _array_element))
        (for _array_element_2 _outactors
          (bind _asbp_base_indicator (Utilities|Casting|CastToBP_BaseIndicator _array_element_2))
          (Utilities|Array|Add (Variables|Horror|GetValidIndicators) _asbp_base_indicator))))))

(fn ConstructionScript)

(fn OnInteract
  (Audio|PlaySound2D (Variables|Horror|GetPressSound) 1.0 1.0 0.0 0 0))

(fn PlayAnimation
  (CallFunction|PlayAnimationEvent))