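; BP_Desinfection is an interactable control button, named for disinfection, that toggles its referenced door open or closed.
; On BeginPlay it finds the BP_Harvester and registers itself as that actor's DesinfectionRef.
; When interacted with while the control is enabled, it opens or closes the door and plays a timeline that sinks the button mesh.
; When the press finishes, RevertControl runs a second timeline in reverse to raise the button.
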(event Custom|RevertControl
  (bind _newtrack_0 (Timeline|Timeline ReverseFromEnd)
    (:Update
      (Transformation|SetRelativeLocation (Variables|Default|GetSM_Button) (Math|Vector|Lerp(Vector) "0.000000,0.000000,-1.000000" "0.000000,0.000000,-3.000000" _newtrack_0) false false))))

(event Custom|OnInteract
  (if (Variables|Default|GetIsControlEnabled)
    (if (Variables|/Game/Blueprints/Harvester/BP_Door.BP_Door_C|GetIsOpen (Variables|Default|GetDoorRef))
      (Default|CloseDoor (Variables|Default|GetDoorRef))
      (bind _newtrack_0 (Timeline|PressTimeline PlayFromStart)
        (:Update
          (Transformation|SetRelativeLocation (Variables|Default|GetSM_Button) (Math|Vector|MakeVector 0.0 0.0 (Math|Float|Lerp -1.0 -3.0 _newtrack_0)) false false))
        (:Finished
          (CallFunction|RevertControl)))
      (else
        (Default|OpenDoor (Variables|Default|GetDoorRef))
        (Timeline|PressTimeline PlayFromStart)))))

(event EventBeginPlay
  (bind _returnvalue (Actor|GetActorOfClass "/Game/Blueprints/Harvester/BP_Harvester.BP_Harvester_C"))
  (bind _output_get (Variables|Default|SetHarvesterRef _returnvalue))
  (Variables|/Game/Blueprints/Harvester/BP_Harvester.BP_Harvester_C|SetDesinfectionRef _output_get self))

(fn ConstructionScript)