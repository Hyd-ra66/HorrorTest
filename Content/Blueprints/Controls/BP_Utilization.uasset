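; BP_Utilization is an interactable disposal unit with a push button and sliding door that destroys the player character's current item.
; Interacting while enabled animates the button press and toggles the door through timelines.
; Closing disables input, then destroys any valid CurrentItem once shut, re-enabling after a short delay, or immediately if none exists.
; SetItem moves that item to the Scene component, and BeginPlay caches a BP_Harvester reference.
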(event Custom|RevertControl
  (bind _newtrack_0 (Timeline|Timeline ReverseFromEnd)
    (:Update
      (Transformation|SetRelativeLocation (Variables|Default|GetSM_Button) (Math|Vector|MakeVector 0.0 0.0 (Math|Float|Lerp -1.0 -3.0 _newtrack_0)) false false))))

(event Custom|OnInteract
  (if (Variables|Default|GetIsEnabled)
    (if (Variables|Default|GetIsOpen)
      (CallFunction|CloseDoor)
      (bind _newtrack_0 (Timeline|PressTimeline PlayFromStart)
        (:Update
          (Transformation|SetRelativeLocation (Variables|Default|GetSM_Button) (Math|Vector|MakeVector 0.0 0.0 (Math|Float|Lerp -1.0 -3.0 _newtrack_0)) false false))
        (:Finished
          (CallFunction|RevertControl)))
      (else
        (CallFunction|OpenDoor)
        (Timeline|PressTimeline PlayFromStart)))))

(event Custom|OpenDoor
  (bind _newtrack_0 (Timeline|Timeline_0 PlayFromStart)
    (:Update
      (Transformation|SetRelativeLocation (Variables|Default|GetDoor) (Math|Vector|MakeVector -5e+01 (Math|Float|Lerp 2.21 -56.0 _newtrack_0) -4.9) false false))
    (:Finished
      (Variables|Default|SetIsOpen true))))

(event Custom|CloseDoor
  (Variables|Default|SetIsEnabled false)
  (bind _newtrack_0 (Timeline|Timeline_1 ReverseFromEnd)
    (:Update
      (Transformation|SetRelativeLocation (Variables|Default|GetDoor) (Math|Vector|MakeVector -5e+01 (Math|Float|Lerp 2.21 -56.0 _newtrack_0) -4.9) false false))
    (:Finished
      (Variables|Default|SetIsOpen false)
      (bind _returnvalue (Actor|GetActorOfClass "/Game/Blueprints/BP_FirstPersonCharacter.BP_FirstPersonCharacter_C"))
      (Utilities|IsValid (Variables|/Game/Blueprints/BP_FirstPersonCharacter.BP_FirstPersonCharacter_C|GetCurrentItem _returnvalue)
        (:Is%20Valid
          (Default|Destroy (Variables|/Game/Blueprints/BP_FirstPersonCharacter.BP_FirstPersonCharacter_C|GetCurrentItem _returnvalue))
          (Utilities|FlowControl|Delay 3.0)
          (Variables|Default|SetIsEnabled true))
        (:Is%20Not%20Valid
          (Variables|Default|SetIsEnabled true))))))

(event Custom|SetItem
  (bind _returnvalue (Actor|GetActorOfClass "/Game/Blueprints/BP_FirstPersonCharacter.BP_FirstPersonCharacter_C"))
  (Default|SetLocation (Variables|/Game/Blueprints/BP_FirstPersonCharacter.BP_FirstPersonCharacter_C|GetCurrentItem _returnvalue) (Variables|Default|GetScene)))

(event EventBeginPlay
  (bind _returnvalue (Actor|GetActorOfClass "/Game/Blueprints/Harvester/BP_Harvester.BP_Harvester_C"))
  (Variables|Default|SetHarvesterRef _returnvalue))

(fn ConstructionScript)