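; BP_BaseIndicator is a base indicator that shows an active or inactive state through the color of a sphere mesh.
; On BeginPlay it creates and stores a dynamic material instance from the sphere, then applies the configured initial state.
; SetState switches the material's Color parameter between the active and inactive colors.
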(event EventBeginPlay
  (bind _returnvalue (Rendering|Material|CreateDynamicMaterialInstance (Variables|Default|GetSphere) 0 0 "None" :!class /Script/Engine.PrimitiveComponent))
  (Variables|Default|SetMID _returnvalue)
  (CallFunction|SetState (Variables|Default|GetInitState)))

(fn ConstructionScript)

(fn SetState
  (params (IsActive :type Boolean))
  (if IsActive
    (Rendering|Material|SetVectorParameterValue (Variables|Default|GetMID) "Color" (Variables|Default|GetActiveColor) :!class /Script/Engine.MaterialInstanceDynamic)
    (else
      (Rendering|Material|SetVectorParameterValue (Variables|Default|GetMID) "Color" (Variables|Default|GetInactiveColor) :!class /Script/Engine.MaterialInstanceDynamic))))