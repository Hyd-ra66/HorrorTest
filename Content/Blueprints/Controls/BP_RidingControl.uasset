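; BP_RidingControl is an interactable control that sinks along Z when its animation plays and can rise back afterward.
; PlayAnimation starts a press timeline that offsets the actor down from its initial location, then switches its valid indicators off.
; Unless a condition is needed to restore it, a delayed reverse timeline raises it again and switches the indicators back on.
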(event EventBeginPlay
  (|CallParentFunction) ; This node is disabled and will not be called.\nDrag off pins to build functionality.
)

(event Collision|EventActorBeginOverlap
  (params (OtherActor :type Actor%20Object%20Reference))
  (|CallParentFunction OtherActor) ; This node is disabled and will not be called.\nDrag off pins to build functionality.
)

(event EventTick
  (params (DeltaSeconds :type Float%20%28single-precision%29))
  (|CallParentFunction DeltaSeconds) ; This node is disabled and will not be called.\nDrag off pins to build functionality.
)

(event EventPlayAnimationEvent
  (bind _initiallocation (Variables|Default|GetInitialLocation))
  (bind _newtrack_0 (Timeline|PressTimeline PlayFromStart)
    (:Update
      (Transformation|SetActorLocation (Math|Vector|MakeVector (.x _initiallocation) (.y _initiallocation) (- (.z _initiallocation) _newtrack_0)) false false))
    (:Finished
      (Utilities|FlowControl|Sequence
        (:then_0
          (for _array_element (Variables|Default|GetValidIndicators)
            (Default|SetState _array_element false)))
        (:then_1
          (if (not (Variables|Default|GetNeedConditionToRestore))
            (CallFunction|PlayReversedAnimation)))))))

(event EventPlayReversedAnimation
  (bind _initiallocation (Variables|Default|GetInitialLocation))
  (Utilities|FlowControl|Delay (Variables|Default|GetDelayBeforeReverseAnimation))
  (bind _newtrack_0 (Timeline|Timeline ReverseFromEnd)
    (:Update
      (Transformation|SetActorLocation (Math|Vector|MakeVector (.x _initiallocation) (.y _initiallocation) (- (.z _initiallocation) _newtrack_0)) false false))
    (:Finished
      (for _array_element (Variables|Default|GetValidIndicators)
        (Default|SetState _array_element true)))))

(fn ConstructionScript
  (|CallParentFunction))

(fn OnInteract
  (|CallParentFunction))

(fn PlayAnimation
  (CallFunction|PlayAnimationEvent))