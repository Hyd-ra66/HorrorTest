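; BP_TravelControl is a pressable control that starts the Harvester's travel.
; On BeginPlay it registers itself with HarvesterRef and switches its indicators on.
; PlayAnimation disables the control and sinks the mesh via a timeline, then turns the indicators off and calls StartTravel on the Harvester.
; RevertControl plays a reverse timeline to raise the mesh, then re-enables the control and its indicators.
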(event Custom|RevertControl
  (bind _newtrack_0 (Timeline|Timeline ReverseFromEnd)
    (:Update
      (Transformation|SetRelativeLocation (Variables|Default|GetStaticMesh) (Math|Vector|Lerp(Vector) "0, 0, 0" (Variables|Default|GetPressedLocation) _newtrack_0) false false))
    (:Finished
      (Variables|Default|SetIsControlEnabled true)
      (for _array_element (Variables|Default|GetValidIndicators)
        (Default|SetState _array_element true)))))

(event EventBeginPlay
  (|CallParentFunction)
  (Variables|/Game/Blueprints/Driving/BP_Harvester.BP_Harvester_C|SetTravelControlRef (Variables|Default|GetHarvesterRef) self)
  (for _array_element (Variables|Default|GetValidIndicators)
    (Default|SetState _array_element true)
    (Variables|Default|SetPressedLocation (Math|Vector|MakeVector 0.0 0.0 -5e+01))))

(event Collision|EventActorBeginOverlap
  (params (OtherActor :type Actor%20Object%20Reference))
  (|CallParentFunction OtherActor) ; This node is disabled and will not be called.\nDrag off pins to build functionality.
)

(event EventTick
  (params (DeltaSeconds :type Float%20%28single-precision%29))
  (|CallParentFunction DeltaSeconds) ; This node is disabled and will not be called.\nDrag off pins to build functionality.
)

(event EventPlayAnimationEvent
  (if (Variables|Default|GetIsControlEnabled)
    (Variables|Default|SetIsControlEnabled false)
    (bind _newtrack_0 (Timeline|PressTimeline PlayFromStart)
      (:Update
        (Transformation|SetRelativeLocation (Variables|Default|GetStaticMesh) (Math|Vector|Lerp(Vector) "0, 0, 0" (Variables|Default|GetPressedLocation) _newtrack_0) false false))
      (:Finished
        (Utilities|FlowControl|Sequence
          (:then_0
            (for _array_element (Variables|Default|GetValidIndicators)
              (Default|SetState _array_element false)))
          (:then_1
            (Default|StartTravel (Variables|Default|GetHarvesterRef))))))))

(fn ConstructionScript
  (|CallParentFunction))

(fn OnInteract
  (|CallParentFunction))

(fn PlayAnimation
  (CallFunction|PlayAnimationEvent))