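; Harvester push-button control that launches a "Zond" probe run and registers itself with the harvester on BeginPlay.
; PlayAnimation locks the control and plays the press timeline, which then starts a delay-scripted sequence of status messages in a W_ZondText widget and calls AnalizeComplete on the harvester.
; A second timeline raises the button as probing begins, re-enabling the control and indicators and setting the decal's inactive color before the sequence ends.
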(event Custom|RevertControl
  ;[0.3033 1 0.3213] RevertButton
  (bind _newtrack_0 (Timeline|Timeline PlayFromStart)
    (:Update
      (Transformation|SetRelativeLocation (Variables|Default|GetSM_Button) (Math|Vector|MakeVector 0.0 0.0 (Math|Float|Lerp -3.0 -1.0 _newtrack_0)) false false))
    (:Finished
      (Utilities|FlowControl|Sequence
        (:then_0
          (Variables|Default|SetIsControlEnabled true)
          (for _array_element (Variables|Default|GetValidIndicators)
            (Default|SetState _array_element true)))
        (:then_1
          (CallFunction|SetDecalState false))))))

(event Custom|StartProbing
  (bind _zondwidget (Variables|Default|GetZondWidget))
  ;[1 0.9568 0.1188] Start probing event
  (CallFunction|CreateWidget)
  (Default|SetText (Variables|Default|GetZondWidget) "Zond is running...")
  (CallFunction|RevertControl)
  (Utilities|FlowControl|Delay 5.0)
  (Default|SetText (Variables|Default|GetZondWidget) "Zond returns")
  (Utilities|FlowControl|Delay 2.0)
  (Default|SetText (Variables|Default|GetZondWidget) "Analizing")
  (Utilities|FlowControl|Delay 5.0)
  (Default|SetText (Variables|Default|GetZondWidget) "Analize complete!")
  (Default|AnalizeComplete (Variables|Default|GetHarvesterRef))
  (Utilities|FlowControl|Delay 2.0)
  (Utilities|IsValid _zondwidget
    (:Is%20Valid
      (Widget|RemovefromParent _zondwidget))))

(event Custom|SetDecalState
  (params (IsActive :type Boolean))
  (if IsActive
    (Rendering|Material|SetVectorParameterValue (Variables|Default|GetDecalMID) "Emissive_Color" (Variables|Default|GetActiveColor) :!class /Script/Engine.MaterialInstanceDynamic)
    (else
      (Rendering|Material|SetVectorParameterValue (Variables|Default|GetDecalMID) "Emissive_Color" (Variables|Default|GetInactiveColor) :!class /Script/Engine.MaterialInstanceDynamic))))

(event EventBeginPlay
  ;[0.2529 1 0.09399] Begin play
  (|CallParentFunction)
  (Variables|/Game/Blueprints/Driving/BP_Harvester.BP_Harvester_C|SetProbingControl (Variables|Default|GetHarvesterRef) self)
  (bind _returnvalue (Rendering|Material|CreateDynamicMaterialInstance (Variables|Default|GetDecal) :!class /Script/Engine.DecalComponent))
  (Variables|Default|SetDecalMID _returnvalue)
  (CallFunction|SetDecalState false)
  (for _array_element (Variables|Default|GetValidIndicators)
    (Default|SetState _array_element true)))

(event Collision|EventActorBeginOverlap
  (params (OtherActor :type Actor%20Object%20Reference))
  (|CallParentFunction OtherActor) ; This node is disabled and will not be called.\nDrag off pins to build functionality.
)

(event EventTick
  (params (DeltaSeconds :type Float%20%28single-precision%29))
  (|CallParentFunction DeltaSeconds) ; This node is disabled and will not be called.\nDrag off pins to build functionality.
)

(event EventPlayAnimationEvent
  ;[0.1667 0.4879 1] Play press animation
  (if (Variables|Default|GetIsControlEnabled)
    (Variables|Default|SetIsControlEnabled false)
    (bind _newtrack_0 (Timeline|PressTimeline PlayFromStart)
      (:Update
        (Transformation|SetRelativeLocation (Variables|Default|GetSM_Button) (Math|Vector|MakeVector 0.0 0.0 (Math|Float|Lerp -1.0 -3.0 _newtrack_0)) false false))
      (:Finished
        (CallFunction|StartProbing)))))

(fn ConstructionScript
  (|CallParentFunction))

(fn OnInteract
  (|CallParentFunction))

(fn PlayAnimation
  (CallFunction|PlayAnimationEvent))

(fn CreateWidget
  (bind _returnvalue (UserInterface|CreateWidget "/Game/Widgets/W_ZondText.W_ZondText_C" (Game|GetPlayerController 0)))
  (bind _output_get (Variables|Default|SetZondWidget _returnvalue))
  (UserInterface|Viewport|AddtoViewport _output_get 0))