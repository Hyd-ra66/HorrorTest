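; Interactable button control that opens the level's door with a single press.
; On BeginPlay it finds the harvester and door by class and registers itself on the harvester.
; Interacting while enabled disables the control, opens the door and plays a timeline that sinks the button mesh.
; RevertControl reverses a separate timeline to raise the button; re-enable, state-toggling and harvester travel logic sit in unconnected nodes.
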(event Custom|RevertControl
  (bind _newtrack_0 (Timeline|Timeline ReverseFromEnd)
    (:Update
      (Transformation|SetRelativeLocation (Variables|Default|GetSM_Button) (Math|Vector|Lerp(Vector) "0.000000,0.000000,-1.000000" "0.000000,0.000000,-3.000000" _newtrack_0) false false))))

(event Custom|OnInteract
  (if (Variables|Default|GetIsControlEnabled)
    (Variables|Default|SetIsControlEnabled false)
    (Default|OpenDoor (Variables|Default|GetDoorRef))
    (bind _newtrack_0 (Timeline|PressTimeline PlayFromStart)
      (:Update
        (Transformation|SetRelativeLocation (Variables|Default|GetSM_Button) (Math|Vector|MakeVector 0.0 0.0 (Math|Float|Lerp -1.0 -3.0 _newtrack_0)) false false)))))

(event EventBeginPlay
  (bind _returnvalue (Actor|GetActorOfClass "/Game/Blueprints/Driving/BP_Harvester.BP_Harvester_C"))
  (Variables|Default|SetHarvesterRef _returnvalue)
  (Variables|/Game/Blueprints/Driving/BP_Harvester.BP_Harvester_C|SetOpenDoorControlRef (Variables|Default|GetHarvesterRef) self)
  (bind _returnvalue_2 (Actor|GetActorOfClass "/Game/Blueprints/Driving/BP_Door.BP_Door_C"))
  (Variables|Default|SetDoorRef _returnvalue_2))

(fn ConstructionScript)